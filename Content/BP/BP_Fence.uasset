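; BP_Fence is a fence that gets knocked loose the first time a MovingOutCharacter overlaps it.
; A DoOnce gates the overlap before the cast, then the mesh starts simulating physics, receives a force and plays a sound at its location.
; The force adds 10000 to the character's forward vector rather than scaling it, so it barely follows the facing direction.
; An AddImpulse alternative is left unconnected.
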(event `self.ReceiveActorBeginOverlap`
  (params (OtherActor :type "Actor Object Reference"))
  (`/Engine/EditorBlueprintResources/StandardMacros.DoOnce` false
    (:`Completed`
      (bind _asmoving_out_character (cast `MovingOutCharacter` OtherActor))
      (`PrimitiveComponent.SetSimulatePhysics` (`self.StaticMesh`) true)
      (`PrimitiveComponent.AddForce` (`self.StaticMesh`) (+ (`self.GetActorForwardVector` _asmoving_out_character) 10000) "None" false)
      (`GameplayStatics.PlaySoundAtLocation` "/Engine/VREditor/Sounds/UI/Drop_Item_From_ContentBrowser.Drop_Item_From_ContentBrowser" (`SceneComponent.K2_GetComponentLocation` (`self.StaticMesh`)) (struct) 1.0 1.0 0.0 "/Game/Sound/BP_OBJSoundAttenuation.BP_OBJSoundAttenuation" null null null))))

(fn `UserConstructionScript`)