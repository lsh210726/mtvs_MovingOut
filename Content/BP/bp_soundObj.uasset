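; Physics object Blueprint that plays an attenuated drop sound at its static mesh when it is knocked or lands.
; Meshes above a mass threshold are checked on Tick for large velocity differences from a stored value, which updates only when that threshold is exceeded.
; Lighter meshes instead trigger on Hit events above a speed threshold.
; Each path uses a delayed DoOnce reset as a cooldown, longer for heavy objects, and prints debug text.
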(event `self.ReceiveTick`
  (params (DeltaSeconds :type "Float (single-precision)"))
  (bind _returnvalue (`KismetMathLibrary.VSize` (- (`SceneComponent.GetComponentVelocity` (`self.StaticMesh`)) (`self.prevVelo`))))
  (bind _returnvalue_2 (`KismetStringLibrary.Conv_DoubleToString` _returnvalue))
  (if (> (`PrimitiveComponent.GetMass` (`self.StaticMesh`)) 50.0)
    (if (> _returnvalue 150.0)
      (`KismetSystemLibrary.PrintString` _returnvalue_2 true true (struct :`G` 0.66 :`B` 1.0 :`A` 1.0) DeltaSeconds)
      (set `self.prevVelo` (`SceneComponent.GetComponentVelocity` (`self.StaticMesh`)))
      (`/Engine/EditorBlueprintResources/StandardMacros.DoOnce` false :!label _label
        (:`Completed`
          (`KismetSystemLibrary.PrintString` "sound")
          (`GameplayStatics.PlaySoundAtLocation` "/Engine/VREditor/Sounds/UI/Drop_Item_From_ContentBrowser.Drop_Item_From_ContentBrowser" (`SceneComponent.K2_GetComponentLocation` (`self.StaticMesh`)) (struct) 1.0 1.0 0.0 "/Game/Sound/BP_OBJSoundAttenuation.BP_OBJSoundAttenuation" null null null)
          (`KismetSystemLibrary.Delay` 2.0)
          (goto _label :!via `Reset`)))
      (else
        (`KismetSystemLibrary.PrintString` _returnvalue_2 true true (struct :`G` 0.66 :`B` 1.0 :`A` 1.0) DeltaSeconds)))))

(event `self.ReceiveHit`
  (params (MyComp :type "PrimitiveComponent Object Reference") (Other :type "Actor Object Reference") (OtherComp :type "PrimitiveComponent Object Reference") (bSelfMoved :type Boolean) (HitLocation :type "Vector Structure") (HitNormal :type "Vector Structure") (NormalImpulse :type "Vector Structure") (Hit :type "HitResult Structure (by ref)"))
  (if (> (`PrimitiveComponent.GetMass` (`self.StaticMesh`)) 50.0)
    _
    (elif (> (`KismetMathLibrary.VSize` (`SceneComponent.GetComponentVelocity` (`self.StaticMesh`))) 300.0)
      (`/Engine/EditorBlueprintResources/StandardMacros.DoOnce` false :!label _label_2
        (:`Completed`
          (`GameplayStatics.PlaySoundAtLocation` "/Engine/VREditor/Sounds/UI/Drop_Item_From_ContentBrowser.Drop_Item_From_ContentBrowser" (`SceneComponent.K2_GetComponentLocation` (`self.StaticMesh`)) (struct) 1.0 1.0 0.0 "/Game/Sound/BP_OBJSoundAttenuation.BP_OBJSoundAttenuation" null null null)
          (`KismetSystemLibrary.PrintString` "sound")
          (`KismetSystemLibrary.Delay` 0.2)
          (goto _label_2 :!via `Reset`))))))

(event `self.ReceiveActorBeginOverlap`
  (params (OtherActor :type "Actor Object Reference")))

(fn `UserConstructionScript`)