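; A shared camera Blueprint that keeps every BP_MovingOutCharacter in the level framed.
; Each Tick it lerps the Sphere toward the players' average location by CamSpeed, without scaling by delta time.
; It sets the SpringArm length to the largest pairwise player distance, clamped between MinCamDist and MaxCamDist.
; An orthographic-width variant of that zoom is left unconnected and never runs.
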(event `self.ReceiveTick`
  (params (DeltaSeconds :type "Float (single-precision)"))
  (set `self.Delta Seconds` DeltaSeconds)
  (set `self.preLocation` (`SceneComponent.K2_GetComponentLocation` (`self.Sphere`)))
  (bind _outactors (`GameplayStatics.GetAllActorsOfClass` "/Game/BP/BP_MovingOutCharacter.BP_MovingOutCharacter_C"))
  (bind _output_get (set `self.players` _outactors))
  (bind _returnvalue (`GameplayStatics.GetActorArrayAverageLocation` _output_get))
  (`SceneComponent.K2_SetWorldLocation` (`self.Sphere`) (`KismetMathLibrary.VLerp` (`self.preLocation`) _returnvalue (`self.camSpeed`)) false false)
  (for (_array_element _array_index) (`self.players`)
    (set `self.player` _array_element)
    (for _index (range (+ _array_index 1) (`KismetArrayLibrary.Array_Length` (`self.players`)))
      (`KismetArrayLibrary.Array_Add` (`self.distance`) (`self.GetDistanceTo` (`self.player`) (`|GetArrayItem` (`self.players`) _index)))))
  (set `SpringArmComponent.TargetArmLength` (`KismetMathLibrary.FClamp` (`.MaxValue` (`KismetMathLibrary.MaxOfFloatArray` (`self.distance`))) (`self.minCamDist`) (`self.maxCamDist`)) (`self.SpringArm`))
  (`KismetArrayLibrary.Array_Clear` (`self.distance`)))

(event `self.ReceiveBeginPlay`)

(fn `UserConstructionScript`)