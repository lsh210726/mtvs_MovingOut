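; Test character that grabs, drags and throws physics bodies, with mouse input routed through server RPC events.
; Left press sphere-traces ahead, then scales walk and turn speed by the grabbed object's mass.
; Objects above LiftMass attach via physics constraint with character rotation locked, while lighter ones follow GrabPosition through a physics handle.
; Left release drops the object and right release throws liftable ones with a forward impulse, both resetting movement.
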(event `self.ReceiveBeginPlay`)

(event `Key|LeftMouseButton`
  (params (Key :type "Key Structure"))
  (:`Pressed`
    (`self.RPC_ServerLeftMousePressed`))
  (:`Released`
    (`self.RPC_ServerLeftMouseReleased`)))

(event `RPC_LeftMouseButtonPressed`
  (bind _returnvalue (`self.K2_GetActorLocation`))
  (bind _returnvalue_2 (`SceneComponent.K2_GetComponentRotation` (`self.Hit Component`)))
  (bind (_rotationrate_roll _rotationrate_pitch _rotationrate_yaw) (`KismetMathLibrary.BreakRotator` (`CharacterMovementComponent.RotationRate` (`self.CharacterMovement`))))
  (bind (_outhit _returnvalue_3) (`KismetSystemLibrary.SphereTraceSingleForObjects` :`Start` _returnvalue :`End` (+ _returnvalue (* (`self.GetActorForwardVector`) 150.0)) :`Radius` 60.0 :`ObjectTypes` (`|MakeArray` "ObjectTypeQuery4" :!type "EObjectTypeQuery Enum") :`DrawTime` 1.0))
  (if _returnvalue_3
    (bind (_bblockinghit _binitialoverlap _time _distance _location _impactpoint _normal _impactnormal _physmat _hitactor _hitcomponent) (`GameplayStatics.BreakHitResult` _outhit))
    (set `self.Hit Component` _hitcomponent)
    (set `self.Impact Point` _impactpoint)
    (if (> (`PrimitiveComponent.GetMass` (`self.Hit Component`)) 11.0)
      (set `self.isGrab` true)
      (set `CharacterMovementComponent.RotationRate` (`KismetMathLibrary.MakeRotator` 0.0 0.0 (/ _rotationrate_yaw (/ (`PrimitiveComponent.GetMass` (`self.Hit Component`)) 50.0))) (`self.CharacterMovement`))
      (set `CharacterMovementComponent.MaxWalkSpeed` (/ (`CharacterMovementComponent.MaxWalkSpeed` (`self.CharacterMovement`)) (/ (`PrimitiveComponent.GetMass` (`self.Hit Component`)) 50.0)) (`self.CharacterMovement`))
      (if (> (`PrimitiveComponent.GetMass` (`self.Hit Component`)) (`self.LiftMass`))
        (`SceneComponent.K2_SetWorldLocation` (`self.Hit Component`) (+ (- (`SceneComponent.K2_GetComponentLocation` (`self.Hit Component`)) (`self.Impact Point`)) (`SceneComponent.K2_GetComponentLocation` (`self.GrabPosition`))) false false)
        (`PhysicsConstraintComponent.SetConstrainedComponents` (`self.PhysicsConstraint`) (`self.CapsuleComponent`) "None" (`self.Hit Component`) "None")
        (`PrimitiveComponent.SetCollisionResponseToChannel` (`self.Hit Component`) "ECC_Pawn" "ECR_Ignore")
        (set `CharacterMovementComponent.bOrientRotationToMovement` false (`self.CharacterMovement`))
        (else
          (set `self.grabRot` _returnvalue_2)
          (`PhysicsHandleComponent.GrabComponentAtLocationWithRotation` (`self.PhysicsHandle`) (`self.Hit Component`) "None" (`SceneComponent.K2_GetComponentLocation` (`self.Hit Component`)) (`KismetMathLibrary.ComposeRotators` _returnvalue_2 (`self.K2_GetActorRotation`)))
          (`PrimitiveComponent.SetCollisionResponseToChannel` (`self.Hit Component`) "ECC_Pawn" "ECR_Ignore"))))))

(event `RPC_ServerLeftMousePressed`
  (`self.RPC_LeftMouseButtonPressed`))

(event `RPC_ServerLeftMouseReleased`
  (`self.RPC_LeftMouseButtonReleased`))

(event `RPC_LeftMouseButtonReleased`
  (if (`self.isGrab`)
    (`PhysicsHandleComponent.ReleaseComponent` (`self.PhysicsHandle`))
    (`PrimitiveComponent.SetCollisionResponseToChannel` (`self.Hit Component`) "ECC_Pawn" "ECR_Block")
    (`PhysicsConstraintComponent.BreakConstraint` (`self.PhysicsConstraint`))
    (set `self.isGrab` false)
    (set `CharacterMovementComponent.RotationRate` (`KismetMathLibrary.MakeRotator` 0.0 0.0 720.0) (`self.CharacterMovement`))
    (set `CharacterMovementComponent.MaxWalkSpeed` 600.0 (`self.CharacterMovement`))
    (set `CharacterMovementComponent.bOrientRotationToMovement` true (`self.CharacterMovement`))))

(event `self.ReceiveTick`
  (params (DeltaSeconds :type "Float (single-precision)"))
  ;[1 1 1] 잡았을 때 물체 위치 지정
  (if (`self.isGrab`)
    (if (> (`PrimitiveComponent.GetMass` (`self.Hit Component`)) (`self.LiftMass`))
      (`self.K2_SetActorRotation` (struct))
      (else
        (`PhysicsHandleComponent.SetTargetLocationAndRotation` (`self.PhysicsHandle`) (`SceneComponent.K2_GetComponentLocation` (`self.GrabPosition`)) (`KismetMathLibrary.ComposeRotators` (`self.K2_GetActorRotation`) (`self.grabRot`)))))))

(event `Key|RightMouseButton`
  (params (Key :type "Key Structure"))
  (:`Released`
    (`self.RPC_ServerRIghtMouseReleased`)))

(event `RPC_ServerRIghtMouseReleased`
  (`self.RPC_RIghtMouseButtonReleased`))

(event `RPC_RIghtMouseButtonReleased`
  (if (`self.isGrab`)
    (if (not (> (`PrimitiveComponent.GetMass` (`self.Hit Component`)) (`self.LiftMass`)))
      (`PhysicsHandleComponent.ReleaseComponent` (`self.PhysicsHandle`))
      (`PrimitiveComponent.AddImpulse` (`self.Hit Component`) (* (`self.GetActorForwardVector`) (`self.ThrowPower`)) "None" false)
      (`PrimitiveComponent.SetCollisionResponseToChannel` (`self.Hit Component`) "ECC_Pawn" "ECR_Block")
      (set `self.isGrab` false)
      (set `CharacterMovementComponent.RotationRate` (`KismetMathLibrary.MakeRotator` 0.0 0.0 360.0) (`self.CharacterMovement`))
      (set `CharacterMovementComponent.MaxWalkSpeed` 600.0 (`self.CharacterMovement`))
      (set `CharacterMovementComponent.bOrientRotationToMovement` true (`self.CharacterMovement`)))))

(fn `UserConstructionScript`)